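; Player controller that switches the player between a flat-screen pawn and a VR pawn, matched to headset state at BeginPlay and toggled with the T debug key.
; ToggleVRMode enables or disables the HMD, then replaces and possesses the pawn at its old transform, or at a player start if none exists.
; VRModeOn updates only when an existing pawn is replaced; switching to VR requires a connected headset.
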(event EventBeginPlay
  (Variables|Default|SetVRModeOn (not (Class|HeadMountedDisplayFunctionLibrary|IsHeadMountedDisplayEnabled)))
  (CallFunction|ToggleVRMode))

(event EventTick
  (params (DeltaSeconds :type Float%20%28single-precision%29)))

(event Input|KeyboardEvents|DebugKeyT
  (params (Key :type Key%20Structure :default "None") (ActionValue :type Input%20Action%20Value%20Structure))
  (:Pressed
    (CallFunction|ToggleVRMode)))

(fn ConstructionScript)

(fn ToggleVRMode
  (bind _returnvalue (Game|Player|GetPlayerPawn 0))
  (bind _returnvalue_2 (Game|Player|GetPlayerPawn 0))
  (if (Variables|Default|GetVRModeOn)
    ;[1 1 1] Turn off VR mode
    (Class|HeadMountedDisplayFunctionLibrary|EnableHMD false)
    (Utilities|IsValid _returnvalue
      (:Is%20Valid
        (LocalVariables|SetOldPawnTransform (Transformation|GetActorTransform _returnvalue))
        (Actor|DestroyActor _returnvalue)
        (bind _returnvalue_3 (Game|SpawnActorfromClass "/Game/FlatPlayer/BP_FlatPlayerPawn.BP_FlatPlayerPawn_C" (LocalVariables|GetOldPawnTransform) "Undefined" "MultiplyWithRoot" 0 0))
        (Pawn|Possess _returnvalue_3)
        (Variables|Default|SetVRModeOn false))
      (:Is%20Not%20Valid
        (bind _returnvalue_4 (Game|SpawnActorfromClass "/Game/FlatPlayer/BP_FlatPlayerPawn.BP_FlatPlayerPawn_C" (Transformation|GetActorTransform (Class|GameModeBase|FindPlayerStart (Game|GetGameMode))) "Undefined" "MultiplyWithRoot" 0 0))
        (Pawn|Possess _returnvalue_4)))
    (elif (Class|HeadMountedDisplayFunctionLibrary|IsHeadMountedDisplayConnected)
      ;[1 1 1] Turn on VR mode
      (Class|HeadMountedDisplayFunctionLibrary|EnableHMD true)
      (Utilities|IsValid _returnvalue_2
        (:Is%20Valid
          (LocalVariables|SetOldPawnTransform (Transformation|GetActorTransform _returnvalue_2))
          (Actor|DestroyActor _returnvalue_2)
          (bind _returnvalue_5 (Game|SpawnActorfromClass "/Game/VRTemplate/Blueprints/VRPawn.VRPawn_C" (LocalVariables|GetOldPawnTransform) "Undefined" "MultiplyWithRoot" 0 0))
          (Pawn|Possess _returnvalue_5)
          (Variables|Default|SetVRModeOn true))
        (:Is%20Not%20Valid
          (bind _returnvalue_6 (Game|SpawnActorfromClass "/Game/VRTemplate/Blueprints/VRPawn.VRPawn_C" (Transformation|GetActorTransform (Class|GameModeBase|FindPlayerStart (Game|GetGameMode))) "Undefined" "MultiplyWithRoot" 0 0))
          (Pawn|Possess _returnvalue_6)))
      (else
        (Development|PrintString "No HMD found!")))))