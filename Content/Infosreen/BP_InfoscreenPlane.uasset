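; Infoscreen plane actor that plays an endless slideshow of PNG images found in a folder under the project directory.
; On BeginPlay it gathers the file names and, if the search succeeds, gives the plane a dynamic instance of M_InfoscreenPlane.
; A self-calling, delayed LoopImages event cycles through the list, importing each file from disk as a texture at runtime and feeding it to the InfoscreenImg parameter.
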(event Custom|LoopImages
  (if (<= (Variables|Default|GetCurrentIndex) (Variables|Default|GetLastIndex))
    _
    (else
      (Variables|Default|SetCurrentIndex 0)))
  (bind _imagepath (CallFunction|GetImagePath (Utilities|Array|Get(acopy) (Variables|Default|GetImageNames) (Variables|Default|GetCurrentIndex))))
  (CallFunction|SetImage _imagepath)
  (Math|Integer|IncrementInt (Variables|Default|GetCurrentIndex)
    (:%20%20
      (Utilities|FlowControl|Delay (Variables|Default|GetImageShowTime))
      (CallFunction|LoopImages))))

(event EventBeginPlay
  (bind _infoscreenplane (Variables|Default|GetInfoscreenPlane))
  (CallFunction|GetImageFolderPath)
  (bind _images_found (CallFunction|GetImageNames))
  (if _images_found
    ;[1 1 1] Sets the material to texture material and creates a dynamic instance of it
    (Rendering|Material|SetMaterial _infoscreenplane 0 "/Game/Infosreen/M_InfoscreenPlane.M_InfoscreenPlane")
    (bind _returnvalue (Rendering|Material|CreateDynamicMaterialInstance _infoscreenplane 0 (Rendering|Material|GetMaterial _infoscreenplane 0) "None" :!class /Script/Engine.PrimitiveComponent))
    (Variables|Default|SetDynamicMaterialInstance _returnvalue)
    (CallFunction|LoopImages)))

(fn ConstructionScript)

(fn GetImageNames
  ;[1 1 1] Gets the file names of the images for later use
  (bind (_foundfiles _returnvalue) (Class|BlueprintFileUtilsBPLibrary|FindFiles (Utilities|String|Append (Class|KismetSystemLibrary|GetProjectDirectory) (Variables|Default|GetImageFolderName)) ".png"))
  (bind _output_get (Variables|Default|SetImageNames _foundfiles))
  (Variables|Default|SetLastIndex (Utilities|Array|LastIndex _output_get))
  (return _returnvalue))

(fn SetImage
  (params (ImagePath :type String))
  (bind _returnvalue (Class|KismetRenderingLibrary|ImportFileasTexture2D ImagePath))
  (Rendering|Material|SetTextureParameterValue (Variables|Default|GetDynamicMaterialInstance) "InfoscreenImg" _returnvalue))

(fn GetImagePath
  (params (ImageName :type String))
  (return (Utilities|String|Append (Variables|Default|GetImageFolderPath) ImageName)))

(fn GetImageFolderPath
  (Variables|Default|SetImageFolderPath (Utilities|String|Append (Class|KismetSystemLibrary|GetProjectDirectory) (Variables|Default|GetImageFolderName))))