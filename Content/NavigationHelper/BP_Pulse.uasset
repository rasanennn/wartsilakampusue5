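; BP_Pulse is a navigation helper actor that travels once along the spline of the wayfinder actor.
; On BeginPlay it finds a BP_WayfinderActor in the level and starts MovePulse.
; A timeline, with play rate set to the inverse of TimeToComplete, lerps distance over the spline's length.
; Each update applies the world location and rotation at that distance, with a fixed non-uniform scale.
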(event Custom|MovePulse
  (bind _splineref (Variables|Default|GetSplineREF))
  (bind _spline (Variables|/Game/NavigationHelper/BP_WayfinderActor.BP_WayfinderActor_C|GetSpline _splineref))
  (Components|Timeline|SetPlayRate (Variables|Default|GetT_MoveObject) (/ 1.0 (Variables|Default|GetTime%20to%20Complete)))
  (bind _move (Timeline|T_MoveObject Play)
    (:Update
      (Transformation|SetActorTransform (Math|Transform|MakeTransform (Spline|GetLocationatDistanceAlongSpline _spline (Math|Float|Lerp 0.0 (Spline|GetSplineLength (Variables|/Game/NavigationHelper/BP_WayfinderActor.BP_WayfinderActor_C|GetSpline (Variables|Default|GetSplineREF))) _move) "World") (Spline|GetRotationatDistanceAlongSpline _spline (Math|Float|Lerp 0.0 (Spline|GetSplineLength (Variables|/Game/NavigationHelper/BP_WayfinderActor.BP_WayfinderActor_C|GetSpline (Variables|Default|GetSplineREF))) _move) "World") "2.500000,0.298640,1.000000")))))

(event EventBeginPlay
  (bind _returnvalue (Actor|GetActorOfClass "/Game/NavigationHelper/BP_WayfinderActor.BP_WayfinderActor_C"))
  (Variables|Default|SetSplineREF _returnvalue)
  (CallFunction|MovePulse))

(fn ConstructionScript)