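; Wayfinder actor that creates and removes a visual for a navmesh route between two locations.
; CreateWayfinderVisual finds the path synchronously, loads its points into a spline and spawns a BP_Pulse at the first point, read in local space.
; DestroyWayfinderVisual removes spline mesh components, clears the spline and destroys the pulse.
; Spline-mesh building in the construction script and create function is disconnected and never runs.
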(event Collision|EventActorBeginOverlap
  (params (OtherActor :type Actor%20Object%20Reference)))

(event EventTick
  (params (DeltaSeconds :type Float%20%28single-precision%29)))

(fn ConstructionScript)

(fn CreateWayfinderVisual
  (params (Start :type Vector) (End :type Vector))
  (bind _returnvalue (Class|NavigationSystemV1|FindPathtoLocationSynchronously Start End (Variables|Default|GetNavMesh) 0))
  (Spline|SetSplinePoints (Variables|Default|GetSpline) (Variables|/Script/NavigationSystem.NavigationPath|GetPathPoints _returnvalue) "World" true)
  (bind _returnvalue_2 (Game|SpawnActorfromClass "/Game/NavigationHelper/BP_Pulse.BP_Pulse_C" (Math|Transform|MakeTransform (Spline|GetLocationatSplinePoint (Variables|Default|GetSpline) 0 "Local") "0, 0, 0" "2.500000,0.298640,1.000000") "AdjustIfPossibleButAlwaysSpawn" "MultiplyWithRoot" 0 0))
  (Variables|Default|SetPulseMesh _returnvalue_2))

(fn DestroyWayfinderVisual
  (bind _arrayelement (Utilities|Array|ReverseforEachLoop (Actor|GetComponentsByClass "/Script/Engine.SplineMeshComponent"))
    (:LoopBody
      (Components|DestroyComponent _arrayelement))
    (:Completed
      (Spline|ClearSplinePoints (Variables|Default|GetSpline) true)
      (Actor|DestroyActor (Variables|Default|GetPulseMesh)))))