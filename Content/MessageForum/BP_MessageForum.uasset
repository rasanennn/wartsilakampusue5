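; Interactable message forum actor whose widget hosts a web browser through which players write messages.
; On BeginPlay it retries on a one-second timer until the browser's bridge object is valid, then binds to its OnMessageSent event.
; Each received message is printed, added to the message array and saved to file through C++ class functions.
; Loading saved messages from file is present but never runs.
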(event Custom|OnMessageSent_Event
  (params (Message :type String))
  (Development|PrintString Message)
  ;[1 1 1] Tämän actorin kanssa vuorovaikutettua pelaaja voi kirjoittaa viestin, joka tallennetaan C++ luokan muuttujien ja functioiden avulla!
  (Class|MessageForum|AddMessagetoArray Message)
  (Class|MessageForum|SaveArraytoFile (Variables|Default|GetAllMessages)))

(event Custom|TryBindMessageEvent
  (bind (_bridgeobject _webbrowserisready) (CallFunction|CheckifBrowserIsReady))
  (if _webbrowserisready
    (EventDispatchers|AssignOnMessageSent _bridgeobject (delegate Custom|OnMessageSent_Event))
    (else
      (Utilities|Time|SetTimerbyEvent (delegate Custom|TryBindMessageEvent) 1.0))))

(event EventBeginPlay
  (CallFunction|TryBindMessageEvent))

(event Collision|EventActorBeginOverlap
  (params (OtherActor :type Actor%20Object%20Reference)))

(event EventTick
  (params (DeltaSeconds :type Float%20%28single-precision%29)))

(fn ConstructionScript)

(fn CheckifBrowserIsReady
  (bind _aswid_message_forum (Utilities|Casting|CastToWid_MessageForum (UserInterface|GetWidget (Variables|Default|GetWidget))))
  (Utilities|IsValid (Variables|/Script/Virtuaalikampus.WebBrowserExtended|GetBridgeObject (Variables|/Game/MessageForum/Wid_MessageForum.Wid_MessageForum_C|GetWebBrowserExtended_79 _aswid_message_forum))
    (:Is%20Valid
      (return (Variables|/Script/Virtuaalikampus.WebBrowserExtended|GetBridgeObject (Variables|/Game/MessageForum/Wid_MessageForum.Wid_MessageForum_C|GetWebBrowserExtended_79 _aswid_message_forum)) true))
    (:Is%20Not%20Valid
      (return (Variables|/Script/Virtuaalikampus.WebBrowserExtended|GetBridgeObject (Variables|/Game/MessageForum/Wid_MessageForum.Wid_MessageForum_C|GetWebBrowserExtended_79 _aswid_message_forum)) false))))

(fn GetWidget
  (return (UserInterface|GetWidget (Variables|Default|GetWidget))))

(fn IsInteractable
  (return true))